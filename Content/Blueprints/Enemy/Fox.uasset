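; Fox enemy character that chases and damages the Egg player and can be hurt or stunned by the Egg's dash.
; AI perception writes Egg visibility to the blackboard and arms the pounce.
; Tick uses Delays to alternate walk speed between pounce bursts and normal movement.
; Hit_Box takes dash damage until death, while Damage_Box either stuns the Fox or damages a non-dashing Egg, with timed cooldowns on damage.
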(event `self.AIPerception.OnTargetPerceptionUpdated`
  (params (Actor :type "Actor Object Reference") (Stimulus :type "AIStimulus Structure"))
  ;[1 1 1] Simple tracking system
  (cast `/Game/Blueprints/Player/Egg` Actor)
  (`BlackboardComponent.SetValueAsBool` (`AIBlueprintHelperLibrary.GetBlackboard` null) "Player_VisableCheck" (`.bSuccessfullySensed` (break `AIStimulus` Stimulus)))
  (set `self.CanPounce` true))

(event `self.Hit_Box.OnComponentBeginOverlap`
  (params (OverlappedComponent :type "PrimitiveComponent Object Reference") (OtherActor :type "Actor Object Reference") (OtherComp :type "PrimitiveComponent Object Reference") (OtherBodyIndex :type Integer) (bFromSweep :type Boolean) (SweepResult :type "HitResult Structure (by ref)"))
  ;[1 1 1] Simple damage mechanic needs to be made more efficient
  (bind _asegg (cast `/Game/Blueprints/Player/Egg` OtherActor))
  (if (`/Game/Blueprints/Player/Egg.Dashing` _asegg)
    (if (`self.Takedamage`)
      (set `self.Takedamage` false)
      (set `self.Health` (- (`self.Health`) 40.0))
      (if (<= (`self.Health`) 0.0)
        (`self.K2_DestroyActor`)
        (else
          (`KismetSystemLibrary.Delay` 2.0)
          (set `self.Takedamage` true)
          (`KismetSystemLibrary.PrintString` "damage dealt"))))))

(event `self.Damage_Box.OnComponentBeginOverlap`
  (params (OverlappedComponent :type "PrimitiveComponent Object Reference") (OtherActor :type "Actor Object Reference") (OtherComp :type "PrimitiveComponent Object Reference") (OtherBodyIndex :type Integer) (bFromSweep :type Boolean) (SweepResult :type "HitResult Structure (by ref)"))
  ;[1 1 1] Stuns the Fox if dashed into/ damages the player if the player isn't dashing
  (bind _asegg (cast `/Game/Blueprints/Player/Egg` OtherActor))
  (if (`/Game/Blueprints/Player/Egg.Dashing` _asegg)
    (set `CharacterMovementComponent.MaxWalkSpeed` (`self.speed`) (`self.CharacterMovement`))
    (set `self.Stunned` true)
    (set `CharacterMovementComponent.RotationRate` (struct) (`self.CharacterMovement`))
    (`KismetSystemLibrary.PrintString` "is stunned 1")
    (`KismetSystemLibrary.Delay` 3.0)
    (set `CharacterMovementComponent.RotationRate` (struct :`Yaw` 180.0) (`self.CharacterMovement`))
    (set `CharacterMovementComponent.MaxWalkSpeed` 600.0 (`self.CharacterMovement`))
    (set `self.Stunned` false)
    (elif (`self.DealDamage`)
      (bind _asegg_2 (cast `/Game/Blueprints/Player/Egg` OtherActor))
      (`/Game/Blueprints/Player/Egg.TakeDamage` _asegg_2 2)
      (set `self.DealDamage` false)
      (`KismetSystemLibrary.Delay` 2.0)
      (set `self.DealDamage` true))))

(event `self.ReceiveTick`
  (params (DeltaSeconds :type "Float (single-precision)"))
  ;[1 1 1] Allows the fox to dash in intervals
  (if (`self.CanPounce`)
    (`KismetSystemLibrary.Delay` (`self.PounceTimer`))
    (set `CharacterMovementComponent.MaxWalkSpeed` (`self.PounceSpeed`) (`self.CharacterMovement`))
    (`KismetSystemLibrary.Delay` 2.0)
    (set `self.CanPounce` false)
    (elif (not (`self.Stunned`))
      (set `CharacterMovementComponent.MaxWalkSpeed` 600.0 (`self.CharacterMovement`))
      (`KismetSystemLibrary.Delay` 3.0)
      (set `self.CanPounce` true))))

(fn `UserConstructionScript`)