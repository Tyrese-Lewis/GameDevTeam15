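; Squirrel enemy that chases the Egg player, hurts it on contact and can be killed by the player's dash.
; AI Perception writes whether the Egg is sensed to a Blackboard bool for the behavior tree.
; Overlapping a dashing Egg reduces Health, and death destroys the squirrel with a random chance to spawn a HealthPickup.
; Box overlap damages a non-dashing Egg, gated by a Delay-based cooldown.
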(event `self.ReceiveActorBeginOverlap`
  (params (OtherActor :type "Actor Object Reference"))
  ;[1 1 1] Handles enemy death
  (bind _asegg (cast `/Game/Blueprints/Player/Egg` OtherActor))
  (if (`/Game/Blueprints/Player/Egg.Dashing` _asegg)
    (set `self.Health` (- (`self.Health`) 40.0))
    (if (<= (`self.Health`) 0.0)
      (`self.K2_DestroyActor`)
      (if (>= (`KismetMathLibrary.RandomFloatInRange` 30.0 100.0) 50.0)
        (`|SpawnActorFromClass` "/Game/Blueprints/HealthPickup.HealthPickup_C" (`self.GetTransform`) "Undefined" "OverrideRootScale" null null)))))

(event `self.AIPerception.OnTargetPerceptionUpdated`
  (params (Actor :type "Actor Object Reference") (Stimulus :type "AIStimulus Structure"))
  ;[1 1 1] If you can see the player update the Behaviour tree (chase)
  (cast `/Game/Blueprints/Player/Egg` Actor)
  (`BlackboardComponent.SetValueAsBool` (`AIBlueprintHelperLibrary.GetBlackboard` null) "Player_VisableCheck" (`.bSuccessfullySensed` (break `AIStimulus` Stimulus))))

(event `self.Box.OnComponentBeginOverlap`
  (params (OverlappedComponent :type "PrimitiveComponent Object Reference") (OtherActor :type "Actor Object Reference") (OtherComp :type "PrimitiveComponent Object Reference") (OtherBodyIndex :type Integer) (bFromSweep :type Boolean) (SweepResult :type "HitResult Structure (by ref)"))
  ;[1 1 1] Damage the player every 2 seconds
  (bind _asegg (cast `/Game/Blueprints/Player/Egg` OtherActor))
  (if (`/Game/Blueprints/Player/Egg.Dashing` _asegg)
    _
    (elif (`self.CanDamage`)
      (bind _asegg_2 (cast `/Game/Blueprints/Player/Egg` OtherActor))
      (`/Game/Blueprints/Player/Egg.TakeDamage` _asegg_2 1)
      (set `self.CanDamage` false)
      (`KismetSystemLibrary.Delay` 2.0)
      (set `self.CanDamage` true))))

(fn `UserConstructionScript`)