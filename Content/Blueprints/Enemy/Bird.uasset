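; Bird enemy that detects the Egg, fires bullets at it and can be killed by the Egg's dash.
; AI perception writes the Egg's sensed state to a blackboard key for a behaviour tree.
; Separately, pawn sensing spawns an Egg_bullet from the muzzle after a fire-rate delay, without the tree.
; Overlapping a dashing Egg subtracts health, destroying the bird at zero or below.
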(event `self.AIPerception.OnTargetPerceptionUpdated`
  (params (Actor :type "Actor Object Reference") (Stimulus :type "AIStimulus Structure"))
  ;[1 1 1] activates the behaviour tree (lock on behaviour tree for ranged models)
  (cast `/Game/Blueprints/Player/Egg` Actor)
  (`BlackboardComponent.SetValueAsBool` (`AIBlueprintHelperLibrary.GetBlackboard` null) "Player_VisableCheck" (`.bSuccessfullySensed` (break `AIStimulus` Stimulus))))

(event `self.PawnSensing.OnSeePawn`
  (params (Pawn :type "Pawn Object Reference"))
  ;[1 1 1] simple lock on and fire mechanic (no behaviour tree)
  (cast `/Game/Blueprints/Player/Egg` Pawn)
  (`KismetSystemLibrary.Delay` (`self.FireRate`))
  (`|SpawnActorFromClass` "/Game/Blueprints/Enemy/Ammo/Egg_bullet.Egg_bullet_C" (`KismetMathLibrary.MakeTransform` (`SceneComponent.K2_GetComponentLocation` (`self.Muzzle`)) (`SceneComponent.K2_GetComponentRotation` (`self.Muzzle`))) "Undefined" "OverrideRootScale" null null))

(event `self.ReceiveActorBeginOverlap`
  (params (OtherActor :type "Actor Object Reference"))
  ;[1 1 1] Simple damage mechanic needs to be made more efficient
  (bind _asegg (cast `/Game/Blueprints/Player/Egg` OtherActor))
  (if (`/Game/Blueprints/Player/Egg.Dashing` _asegg)
    (`KismetSystemLibrary.PrintString` "damage dealt")
    (set `self.Health` (- (`self.Health`) 40.0))
    (if (<= (`self.Health`) 0.0)
      (`self.K2_DestroyActor`))
    (else
      (`KismetSystemLibrary.PrintString` "Not dashing"))))

(fn `UserConstructionScript`)